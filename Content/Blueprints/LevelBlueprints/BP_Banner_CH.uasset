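; BP_Banner_CH is a construction-time banner that lays spline meshes along an editable spline.
; For each pair of neighboring spline points, it adds a segment fitted to their local positions and tangents.
; Each segment gets a random color by shuffling the color array and setting the "Color" material parameter.
; Thickness drives the root's Y and Z scale, with X fixed, and the event graph has no active logic.
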(fn `UserConstructionScript`
  (bind _spline (`self.Spline`))
  (bind _defaultsceneroot (`self.DefaultSceneRoot`))
  (bind _thickness (`self.Thickness`))
  (bind _colorparameter (`self.ColorParameter`))
  (for _index (range (+ (- (`SplineComponent.GetNumberOfSplinePoints` _spline) 2) 1))
    (bind _returnvalue (`AddComponent|NODE_AddSplineMeshComponent-0`))
    (`KismetArrayLibrary.Array_Shuffle` _colorparameter)
    (`MeshComponent.SetVectorParameterValueOnMaterials` _returnvalue "Color" (`|GetArrayItem` _colorparameter))
    (`SceneComponent.K2_AttachToComponent` _returnvalue _defaultsceneroot "None" "KeepRelative" "KeepRelative" "KeepRelative" true)
    (bind (_location _tangent) (`SplineComponent.GetLocationAndTangentAtSplinePoint` _spline _index "Local"))
    (bind (_location_2 _tangent_2) (`SplineComponent.GetLocationAndTangentAtSplinePoint` _spline (+ _index 1) "Local"))
    (`SplineMeshComponent.SetStartAndEnd` _returnvalue _location _tangent _location_2 _tangent_2 true)
    (`SceneComponent.SetRelativeScale3D` _defaultsceneroot (`KismetMathLibrary.MakeVector` 2.0 _thickness _thickness))))