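; Base pickup actor for non-weapon power-ups that spins and, on server overlap, grants its power-up to a character without one already active.
; On pickup it plays a sound, hides itself, removes its trigger sphere, then after a delay spawns a replacement balloon and destroys itself.
; Hits from anything not tagged Projectile switch off physics and collision, so bullets don't leave it stuck in mid-air.
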(event `SpawnBalloonThenDestroy`
  (bind (_returnvalue_location _returnvalue_rotation) (`KismetMathLibrary.BreakTransform` (`KismetMathLibrary.Conv_VectorToTransform` (+ (`self.K2_GetActorLocation`) (`self.BalloonSpawnLocation`)))))
  ;[1 1 1] Respawns Power Up Balloon
  (`/Engine/EditorBlueprintResources/ActorMacros.Switch Has Authority`
    (:`Authority`
      (`SceneComponent.SetHiddenInGame` (`self.PhysicsCollision`) true true)
      (`SceneComponent.SetHiddenInGame` (`self.StaticMesh`) true true)
      (`ActorComponent.K2_DestroyComponent` (`self.Sphere`))
      (`KismetSystemLibrary.Delay` (`self.BalloonTimeRespawn`))
      (`|SpawnActorFromClass` "/Game/Blueprints/Powerups/BP_PowerupBalloon-CS.BP_PowerupBalloon-CS_C" (`KismetMathLibrary.MakeTransform` _returnvalue_location _returnvalue_rotation (4.0 4.0 4.0)) "Undefined" "OverrideRootScale" null null)
      (`self.K2_DestroyActor`))
    (:`Remote`
      (`SceneComponent.SetHiddenInGame` (`self.PhysicsCollision`) true true)
      (`SceneComponent.SetHiddenInGame` (`self.StaticMesh`) true true))))

(event `self.ReceiveBeginPlay`
  ;[1 1 1] Rotates Mesh
  (`KismetSystemLibrary.K2_SetTimer` null "RotateObject" 0.01 true))

(event `RotateObject`
  ;[1 1 1] Rotates Mesh
  (`SceneComponent.K2_AddLocalRotation` (`self.PhysicsCollision`) (struct :`Yaw` 2.0) false false))

(event `PlayPickupSoundEffect`
  ;[0.2224 1 0.1893] Sound Effect
  (`GameplayStatics.PlaySoundAtLocation` (`self.Sound`) (`self.K2_GetActorLocation`)))

(event `self.Sphere.OnComponentBeginOverlap`
  (params (OverlappedComponent :type "PrimitiveComponent Object Reference") (OtherActor :type "Actor Object Reference") (OtherComp :type "PrimitiveComponent Object Reference") (OtherBodyIndex :type Integer) (bFromSweep :type Boolean) (SweepResult :type "HitResult Structure (by ref)"))
  ;[1 1 1] Checks if player has collided / activates power up bool / sets power up enum
  (`/Engine/EditorBlueprintResources/ActorMacros.Switch Has Authority`
    (:`Authority`
      (bind _ash2o_default_third_person_character (cast `/Game/Blueprints/Characters/H2O_Default_ThirdPersonCharacter` OtherActor))
      (if (not (`/Game/Blueprints/Characters/H2O_Default_ThirdPersonCharacter.HasActivePowerup?` _ash2o_default_third_person_character))
        (set `/Game/Blueprints/Characters/H2O_Default_ThirdPersonCharacter.MyNonWeaponPowerups` (`self.NonWeaponPowerup`) _ash2o_default_third_person_character)
        (set `/Game/Blueprints/Characters/H2O_Default_ThirdPersonCharacter.HasActivePowerup?` true _ash2o_default_third_person_character)
        (`/Game/Blueprints/Characters/H2O_Default_ThirdPersonCharacter.ServerSetNonWeaponPowerups` _ash2o_default_third_person_character)
        (`KismetSystemLibrary.K2_ClearTimer` null "RotateObject")
        (`self.SpawnBalloonThenDestroy`)
        (`self.PlayPickupSoundEffect`)))))

(event `self.PhysicsCollision.OnComponentHit`
  (params (HitComponent :type "PrimitiveComponent Object Reference") (OtherActor :type "Actor Object Reference") (OtherComp :type "PrimitiveComponent Object Reference") (NormalImpulse :type "Vector Structure") (Hit :type "HitResult Structure (by ref)"))
  (bind _physicscollision (`self.PhysicsCollision`))
  ;[1 1 1] Checks if Bullets Hits the collider / Stops powerup from staying stuck in mid hair from bullet collision
  (`/Engine/EditorBlueprintResources/ActorMacros.Switch Has Authority`
    (:`Authority`
      _)
    (:`Remote`
      _))
  (if (not (`ActorComponent.ComponentHasTag` (`Actor.RootComponent` OtherActor) "Projectile"))
    (`PrimitiveComponent.SetSimulatePhysics` _physicscollision false)
    (`PrimitiveComponent.SetCollisionEnabled` _physicscollision "NoCollision")
    (`PrimitiveComponent.SetCollisionResponseToAllChannels` _physicscollision "ECR_Ignore")))

(fn `UserConstructionScript`)