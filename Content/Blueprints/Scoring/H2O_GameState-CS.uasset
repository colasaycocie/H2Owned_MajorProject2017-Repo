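; Game State that watches every player's score and triggers the win sequence when one equals the max score to win.
; A looping timer started on BeginPlay polls each player state's score in place of Tick.
; Winning clears the timer, slows time, fades player cameras to black, then restores speed after a delay and prints a placeholder for win logic.
; Score-reset and timer-restart logic exists but is unconnected.
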(event `WinGame`
  ;[1 1 1] Clears Checkscore Timer / Slows down time
  (`KismetSystemLibrary.K2_ClearTimer` null "CheckScore") ; Clears Check Score Timer
  (`GameplayStatics.SetGlobalTimeDilation` 0.2) ; Slow downs time
  ;[1 1 1] Camera Fade to all players
  (for (_ _array_index) (`GameStateBase.PlayerArray` (`GameplayStatics.GetGameState`))
    (bind _ash20_default_third_person_player_controller (cast `/Game/Blueprints/Gameplay/H20_DefaultThirdPersonPlayerController` (`GameplayStatics.GetPlayerController` _array_index)))
    (`PlayerCameraManager.StartCameraFade` (`PlayerController.PlayerCameraManager` _ash20_default_third_person_player_controller) 0.0 2.0 2.0 (struct :`A` 1.0) false false)
    ;[1 1 1] Slow down time set back to normal / Win game logic
    (`KismetSystemLibrary.Delay` 1.0)
    (`GameplayStatics.SetGlobalTimeDilation` 1.0) ; Sets slow time to normal
    (`KismetSystemLibrary.PrintString` "WON GAME - Set up logic in \"GameState-CS\"")))

(event `self.ReceiveBeginPlay`
  ;[1 1 1] Checks if Player Score is at Max Score every .1 second. - Like using Event Tick but not
  (`KismetSystemLibrary.K2_SetTimer` null "CheckScore" 0.1 true))

(event `CheckScore`
  ;[1 0.2734 0.1335] Checks All plays Score
  (for _array_element (`GameStateBase.PlayerArray` (`GameplayStatics.GetGameState`))
    (bind _ash2o_player_state__cs (cast `/Game/Blueprints/Scoring/H2O_PlayerState-CS` _array_element))
    (if (== (`/Game/Blueprints/Scoring/H2O_PlayerState-CS.PlayerScore` _ash2o_player_state__cs) (`self.MaxScoreToWin`))
      (`self.WinGame`))))

(fn `UserConstructionScript`)