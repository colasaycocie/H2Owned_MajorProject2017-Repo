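; VFX test water gun that auto-fires bubble splatter and shooting emitters from BeginPlay on a delayed loop until ammo runs out.
; The loop drains the tank material's FillAmount, while Tick feeds averaged horizontal velocity into its ObjectVelocity parameter.
; Splatter particle deaths play a quiet pop sound.
; TestFire and OnRep_isShooting hold temporary, authority-only projectile spawning aimed by player 0's camera, marked for removal.
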(event `self.ReceiveBeginPlay`
  (bind _particlesystem (`self.ParticleSystem`))
  (bind _splatter (`self.Splatter`))
  (bind _ammo (`self.Ammo`))
  (set `self.Ammo` 100.0)
  (if (> _ammo 0.0) :!label _label
    (`MeshComponent.SetScalarParameterValueOnMaterials` (`self.TankInner`) "FillAmount" (/ _ammo 100.0))
    (set `self.Ammo` (- _ammo 1.0))
    (`GameplayStatics.SpawnEmitterAtLocation` "/Game/VFX/WaterGun/VFX_SYS_BubbleSplatter01_LH.VFX_SYS_BubbleSplatter01_LH" (`SceneComponent.K2_GetComponentLocation` _splatter) (`SceneComponent.K2_GetComponentRotation` _splatter))
    (`GameplayStatics.SpawnEmitterAtLocation` "/Game/VFX/WaterGun/Shooting/VFX_SYS_Shooting_LH.VFX_SYS_Shooting_LH" (`SceneComponent.K2_GetComponentLocation` _particlesystem) (`SceneComponent.K2_GetComponentRotation` _particlesystem))
    (`KismetSystemLibrary.Delay` 1.5)
    (goto _label)))

(event `self.Splatter.OnParticleDeath`
  (params (EventName :type Name) (EmitterTime :type "Float (single-precision)") (ParticleTime :type Integer) (Location :type "Vector Structure") (Velocity :type "Vector Structure") (Direction :type "Vector Structure"))
  (`GameplayStatics.PlaySoundAtLocation` "/Game/Assets/Audio/Powerups/PowerupBalloonPop/H2O_SFX_FloatingBalloonPop_24_v1_MSTD_PS.H2O_SFX_FloatingBalloonPop_24_v1_MSTD_PS" Location (struct) 0.01))

(event `self.ReceiveTick`
  (params (DeltaSeconds :type "Float (single-precision)"))
  (bind (_returnvalue_x _returnvalue_y) (`KismetMathLibrary.BreakVector` (`self.GetVelocity`)))
  (`MeshComponent.SetScalarParameterValueOnMaterials` (`self.TankInner`) "ObjectVelocity" (/ (+ _returnvalue_x _returnvalue_y) 2.0)))

(fn `OnRep_isShooting`
  (bind _ash2o_default_third_person_character (cast `/Game/Blueprints/Characters/H2O_Default_ThirdPersonCharacter` (`GameplayStatics.GetPlayerCharacter` 0) :!pure true))
  (bind _returnvalue (`SceneComponent.K2_GetComponentRotation` (`/Game/Blueprints/Characters/H2O_Default_ThirdPersonCharacter.ThirdPersonCamera` _ash2o_default_third_person_character)))
  ;[1 1 1] This will be removed
  (`/Engine/EditorBlueprintResources/ActorMacros.Switch Has Authority`
    (:`Authority`
      (`|SpawnActorFromClass` "/Game/Blueprints/Weapons/BP_MachineGunProjectile.BP_MachineGunProjectile_C" (`KismetMathLibrary.MakeTransform` (+ (`SceneComponent.K2_GetComponentLocation` (`Character.CapsuleComponent` _ash2o_default_third_person_character)) (`KismetMathLibrary.GreaterGreater_VectorRotator` (100.0 0.0 50.0) _returnvalue)) _returnvalue) "Undefined" "OverrideRootScale" null null))))

(fn `TestFire`
  (bind _ash2o_default_third_person_character (cast `/Game/Blueprints/Characters/H2O_Default_ThirdPersonCharacter` (`GameplayStatics.GetPlayerCharacter` 0) :!pure true))
  (bind _returnvalue (`SceneComponent.K2_GetComponentRotation` (`/Game/Blueprints/Characters/H2O_Default_ThirdPersonCharacter.ThirdPersonCamera` _ash2o_default_third_person_character)))
  ;[1 1 1] This will be removed
  (`/Engine/EditorBlueprintResources/ActorMacros.Switch Has Authority`
    (:`Authority`
      (`|SpawnActorFromClass` "/Game/Blueprints/Weapons/BP_MachineGunProjectile.BP_MachineGunProjectile_C" (`KismetMathLibrary.MakeTransform` (+ (`SceneComponent.K2_GetComponentLocation` (`Character.CapsuleComponent` _ash2o_default_third_person_character)) (`KismetMathLibrary.GreaterGreater_VectorRotator` (100.0 0.0 50.0) _returnvalue)) _returnvalue) "Undefined" "OverrideRootScale" null null))))

(fn `UserConstructionScript`)