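; H20_DefaultPlayerController is a player controller with an unfinished respawn flow, noted as not working for clients.
; Respawn checks for a controlled pawn, printing a debug message if one exists and otherwise calling RequestGMRespawn.
; That event acts only with authority, asking H2O_DefaultGameMode to respawn player controller index 0 rather than the calling controller.
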(event `Respawn`
  ;[0.8103 0.08215 0.0499] Respawning - Not working, Client still doesnt respawn
  (`/Engine/EditorBlueprintResources/ActorMacros.Switch Has Authority`
    (:`Authority`
      _)
    (:`Remote`
      _))
  (`/Engine/EditorBlueprintResources/StandardMacros.IsValid` (`self.K2_GetPawn`)
    (:`Is Valid`
      (`KismetSystemLibrary.PrintString` "PC Class still has pawn controlled "))
    (:`Is Not Valid`
      (`self.requestGMRespawn`)
      (`KismetSystemLibrary.PrintString` "Respawned"))))

(event `requestGMRespawn`
  (bind _returnvalue (`GameplayStatics.GetGameMode`))
  ;[0.8103 0.08215 0.0499] Respawning - Not working, Client still doesnt respawn
  (`/Engine/EditorBlueprintResources/ActorMacros.Switch Has Authority`
    (:`Authority`
      (`/Engine/EditorBlueprintResources/StandardMacros.IsValid` _returnvalue
        (:`Is Valid`
          (bind _ash2o_default_game_mode (cast `/Game/Blueprints/H2O_DefaultGameMode` _returnvalue))
          (`/Engine/EditorBlueprintResources/StandardMacros.IsValid` _ash2o_default_game_mode
            (:`Is Valid`
              (bind _ash20_default_player_controller (cast `/Game/Blueprints/H20_DefaultPlayerController` (`GameplayStatics.GetPlayerController` 0)))
              (`/Game/Blueprints/H2O_DefaultGameMode.Respawn` _ash2o_default_game_mode _ash20_default_player_controller))))))))

(fn `UserConstructionScript`)