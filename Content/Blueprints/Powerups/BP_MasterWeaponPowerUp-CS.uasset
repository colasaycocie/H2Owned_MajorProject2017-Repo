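; Master weapon power-up pickup that grants a weapon type to an H2O third-person character on overlap.
; A looping timer spins the pickup, and its physics body stops simulating and disables collision once it hits something.
; Overlap runs on the server only: if the character has no active power-up, it sets the weapon type, flags the power-up, resets the weapon mesh and destroys itself.
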(event `RotateObject`
  (`SceneComponent.K2_AddLocalRotation` (`self.PhysicsCollision`) (struct :`Yaw` 2.0) false false))

(event `self.ReceiveBeginPlay`
  (`KismetSystemLibrary.K2_SetTimer` null "RotateObject" 0.01 true))

(event `self.Sphere.OnComponentBeginOverlap`
  (params (OverlappedComponent :type "PrimitiveComponent Object Reference") (OtherActor :type "Actor Object Reference") (OtherComp :type "PrimitiveComponent Object Reference") (OtherBodyIndex :type Integer) (bFromSweep :type Boolean) (SweepResult :type "HitResult Structure (by ref)"))
  (`/Engine/EditorBlueprintResources/ActorMacros.Switch Has Authority`
    (:`Authority`
      (bind _ash2o_default_third_person_character (cast `/Game/Blueprints/Characters/H2O_Default_ThirdPersonCharacter` OtherActor))
      (if (not (`/Game/Blueprints/Characters/H2O_Default_ThirdPersonCharacter.HasActivePowerup?` _ash2o_default_third_person_character))
        (set `/Game/Blueprints/Characters/H2O_Default_ThirdPersonCharacter.MyWeaponTypes` (`self.WeaponPowerupType`) _ash2o_default_third_person_character)
        (set `/Game/Blueprints/Characters/H2O_Default_ThirdPersonCharacter.HasActivePowerup?` true _ash2o_default_third_person_character)
        (`/Game/Blueprints/Characters/H2O_Default_ThirdPersonCharacter.ServerResetWeaponMesh` _ash2o_default_third_person_character)
        (`KismetSystemLibrary.K2_ClearTimer` null "RotateObject")
        (`self.K2_DestroyActor`)))))

(event `self.PhysicsCollision.OnComponentHit`
  (params (HitComponent :type "PrimitiveComponent Object Reference") (OtherActor :type "Actor Object Reference") (OtherComp :type "PrimitiveComponent Object Reference") (NormalImpulse :type "Vector Structure") (Hit :type "HitResult Structure (by ref)"))
  (bind _physicscollision (`self.PhysicsCollision`))
  (`PrimitiveComponent.SetSimulatePhysics` _physicscollision false)
  (`PrimitiveComponent.SetCollisionEnabled` _physicscollision "NoCollision")
  (`PrimitiveComponent.SetCollisionResponseToAllChannels` _physicscollision "ECR_Ignore"))

(fn `UserConstructionScript`)