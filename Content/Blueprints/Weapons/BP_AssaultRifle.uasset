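; Assault rifle weapon Blueprint that fires water gun projectiles.
; Its Fire event calls FullyAutomaticAR, which on authority spawns an explosion emitter and a single projectile at the mesh's Muzzle socket.
; WeaponFire and StopWeaponFire are empty, and the looping fire-rate timer meant for automatic fire is disconnected, as is a call to the player character's BeginShoot.
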(event `Fire`
  (`self.FullyAutomaticAR`))

(event `self.WeaponFire`)

(event `self.StopWeaponFire`)

(fn `FullyAutomaticAR`
  (bind _staticmesh (`self.StaticMesh`))
  (`/Engine/EditorBlueprintResources/ActorMacros.Switch Has Authority`
    (:`Authority`
      (`GameplayStatics.SpawnEmitterAtLocation` "/Game/StarterContent/Particles/P_Explosion.P_Explosion" (`SceneComponent.GetSocketLocation` _staticmesh "Muzzle"))
      (`|SpawnActorFromClass` "/Game/Blueprints/Weapons/BP_WaterGunProjectile.BP_WaterGunProjectile_C" (`SceneComponent.GetSocketTransform` _staticmesh "Muzzle" "RTS_World") "Undefined" "OverrideRootScale"))))

(fn `UserConstructionScript`
  (`parent.UserConstructionScript`))