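; Main menu GameMode that prepares the player's persistent profile in the PlayerSettingsSave slot.
; On BeginPlay it caches the GameInfoInstance, then loads PlayerInfo from the slot or creates a save if none exists.
; It then stamps PlayerInfo with the first PlayerState's name and saves again.
; SaveGame lazily creates the PlayerSaveGame object, as LoadGame copies only the struct without keeping the loaded object.
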(event `self.ReceiveBeginPlay`
  (bind _asgame_info_instance (cast `/Game/Blueprints/AllLevels/GameInfoInstance` (`GameplayStatics.GetGameInstance`)))
  (set `self.GameInstanceRef` _asgame_info_instance)
  (`self.SaveGameCheck`)
  (setmembers `/Game/Blueprints/AllLevels/PlayerInfo` :`StructRef` (`self.PlayerInfo`) :`MyPlayerName` (`KismetTextLibrary.Conv_StringToText` (`PlayerState.PlayerName` (`|GetArrayItem` (`GameStateBase.PlayerArray` (`GameplayStatics.GetGameState`))))))
  (`self.SaveGame`))

(fn `LoadGame`
  (bind _returnvalue (`GameplayStatics.LoadGameFromSlot` (`self.PlayerSettingsSave`)))
  (bind _asplayer_save_game (cast `/Game/Blueprints/AllLevels/PlayerSaveGame` _returnvalue))
  (set `self.PlayerInfo` (`/Game/Blueprints/AllLevels/PlayerSaveGame.S_PlayerInfo` _asplayer_save_game)))

(fn `SaveGame`
  (bind _savegameref (`self.SaveGameRef`))
  (`/Engine/EditorBlueprintResources/StandardMacros.IsValid` (`self.SaveGameRef`)
    (:`Is Valid`
      _)
    (:`Is Not Valid`
      (bind _returnvalue (`GameplayStatics.CreateSaveGameObject` "/Game/Blueprints/AllLevels/PlayerSaveGame.PlayerSaveGame_C"))
      (bind _asplayer_save_game (cast `/Game/Blueprints/AllLevels/PlayerSaveGame` _returnvalue))
      (set `self.SaveGameRef` _asplayer_save_game)))
  (set `/Game/Blueprints/AllLevels/PlayerSaveGame.S_PlayerInfo` (`self.PlayerInfo`) _savegameref)
  (`GameplayStatics.SaveGameToSlot` _savegameref (`self.PlayerSettingsSave`)))

(fn `SaveGameCheck`
  (bind _returnvalue (`GameplayStatics.DoesSaveGameExist` (`self.PlayerSettingsSave`)))
  (if _returnvalue
    (`self.LoadGame`)
    (else
      (`self.SaveGame`))))

(fn `UserConstructionScript`)