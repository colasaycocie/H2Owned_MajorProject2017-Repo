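; BP_ReloadTrigger is a trigger actor that marks where players are able to reload.
; On the server, its sphere sets CanReload to true on an overlapping H2O_Default_ThirdPersonCharacter and back to false when the overlap ends.
; Every tick, its text label copies the rotation of player controller 0 and adds a 180-degree local turn to face the camera.
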(event `self.Sphere.OnComponentBeginOverlap`
  (params (OverlappedComponent :type "PrimitiveComponent Object Reference") (OtherActor :type "Actor Object Reference") (OtherComp :type "PrimitiveComponent Object Reference") (OtherBodyIndex :type Integer) (bFromSweep :type Boolean) (SweepResult :type "HitResult Structure (by ref)"))
  ;[1 1 1] Checks if Player is overlapping and is able to reload
  (`/Engine/EditorBlueprintResources/ActorMacros.Switch Has Authority`
    (:`Authority`
      (bind _ash2o_default_third_person_character (cast `/Game/Blueprints/Characters/H2O_Default_ThirdPersonCharacter` OtherActor))
      (set `/Game/Blueprints/Characters/H2O_Default_ThirdPersonCharacter.CanReload?` true _ash2o_default_third_person_character))))

(event `self.Sphere.OnComponentEndOverlap`
  (params (OverlappedComponent :type "PrimitiveComponent Object Reference") (OtherActor :type "Actor Object Reference") (OtherComp :type "PrimitiveComponent Object Reference") (OtherBodyIndex :type Integer))
  ;[1 1 1] Checks if Player is overlapping and is able to reload
  (`/Engine/EditorBlueprintResources/ActorMacros.Switch Has Authority`
    (:`Authority`
      (bind _ash2o_default_third_person_character (cast `/Game/Blueprints/Characters/H2O_Default_ThirdPersonCharacter` OtherActor))
      (set `/Game/Blueprints/Characters/H2O_Default_ThirdPersonCharacter.CanReload?` false _ash2o_default_third_person_character))))

(event `self.ReceiveTick`
  (params (DeltaSeconds :type "Float (single-precision)"))
  (bind _textrender (`self.TextRender`))
  ;[1 1 1] Rotates Text to look at camera
  (`SceneComponent.K2_SetWorldRotation` _textrender (.rotation (`self.GetTransform` (`GameplayStatics.GetPlayerController` 0))) false false)
  (`SceneComponent.K2_AddLocalRotation` _textrender (struct :`Yaw` 180.0) false false))

(fn `UserConstructionScript`)