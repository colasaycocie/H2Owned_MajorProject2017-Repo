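; Pool water hazard that spawns splash and ripple effects at the water surface and damages players who enter it.
; On overlap, it compares the other actor against player pawns via the GameState PlayerArray.
; Players get a player splash and damage; anything else is treated as ammo with its own splash.
; PlayerHit is never reset here, so once set, later overlaps also take the player branch.
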(event `self.PoolWater.OnComponentBeginOverlap`
  (params (OverlappedComponent :type "PrimitiveComponent Object Reference") (OtherActor :type "Actor Object Reference") (OtherComp :type "PrimitiveComponent Object Reference") (OtherBodyIndex :type Integer) (bFromSweep :type Boolean) (SweepResult :type "HitResult Structure (by ref)"))
  (bind (_returnvalue_x _returnvalue_y) (`KismetMathLibrary.BreakVector` (`self.K2_GetActorLocation` OtherActor)))
  (bind (_returnvalue_x_2 _returnvalue_y_2 _returnvalue_z) (`KismetMathLibrary.BreakVector` (`SceneComponent.K2_GetComponentLocation` (`self.PoolWater`))))
  (bind _returnvalue (`KismetMathLibrary.MakeVector` _returnvalue_x _returnvalue_y (+ 1.0 _returnvalue_z)))
  (for (_ _array_index) (`GameStateBase.PlayerArray` (`GameplayStatics.GetGameState`))
    (if (== OtherActor (`GameplayStatics.GetPlayerPawn` _array_index))
      (set `self.PlayerHit` true)))
  (if (`self.PlayerHit`)
    ;[1 1 1] Player hits the pool
    (`GameplayStatics.SpawnEmitterAtLocation` "/Game/VFX/Pool/VFX_SYS_PlayerSplash01_LH.VFX_SYS_PlayerSplash01_LH" _returnvalue)
    (`GameplayStatics.SpawnEmitterAtLocation` "/Game/VFX/Pool/VFX_SYS_Ripple01_LH.VFX_SYS_Ripple01_LH" _returnvalue)
    (`GameplayStatics.ApplyDamage` OtherActor 100.0 null self)
    (else
      ;[1 1 1] Ammo hits the pool
      (`GameplayStatics.SpawnEmitterAtLocation` "/Game/VFX/Pool/VFX_SYS_AmmoSplash01_LH.VFX_SYS_AmmoSplash01_LH" _returnvalue)
      (`GameplayStatics.SpawnEmitterAtLocation` "/Game/VFX/Pool/VFX_SYS_Ripple01_LH.VFX_SYS_Ripple01_LH" _returnvalue))))

(fn `UserConstructionScript`)