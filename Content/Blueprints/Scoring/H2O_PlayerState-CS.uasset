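; H2O_PlayerState is a player state Blueprint that tracks a player's score and death count.
; Two functions, IncrementPlayerScore and IncrementPlayerDeath, each add one to their counter.
; The event graph and construction script do no work; leftover debug prints of name, deaths and score are never run.
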(event `self.ReceiveTick`
  (params (DeltaSeconds :type "Float (single-precision)")))

(fn `IncrementPlayerDeath`
  (set `self.PlayerDeath` (+ (`self.PlayerDeath`) 1)))

(fn `IncrementPlayerScore`
  (set `self.PlayerScore` (+ (`self.PlayerScore`) 1)))

(fn `UserConstructionScript`)