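; Water shotgun projectile whose short lifespan caps its range and which bursts on hit.
; On the server, a hit applies flat damage to pawns and destructibles in a sphere overlap, then spawns the explosion effect, disables collision and shortens remaining life.
; For direct hits on living characters, the locally controlled shooter gets a hit marker, plus a hit sound unless the victim's KillPlayer flag is set.
; The explosion sound is unwired.
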(event `self.ReceiveBeginPlay`
  ;[1 1 1] Distance
  (`self.SetLifeSpan` 0.6) ; Distance
)

(event `self.SphereCollision.OnComponentHit`
  (params (HitComponent :type "PrimitiveComponent Object Reference") (OtherActor :type "Actor Object Reference") (OtherComp :type "PrimitiveComponent Object Reference") (NormalImpulse :type "Vector Structure") (Hit :type "HitResult Structure (by ref)"))
  (bind _returnvalue (`self.GetInstigator`))
  (bind _returnvalue_2 (`Pawn.GetController` _returnvalue))
  ;[1 1 1] Damage Logic
  (`/Engine/EditorBlueprintResources/ActorMacros.Switch Has Authority`
    (:`Authority`
      (`self.OnWaterBombLive`))
    (:`Remote`
      _))
  ;[1 1 1] Checks if can spawn Hitmarker UI
  (bind _ash2o_default_third_person_character (cast `/Game/Blueprints/Characters/H2O_Default_ThirdPersonCharacter` OtherActor))
  (if (not (`/Game/Blueprints/Characters/H2O_Default_ThirdPersonCharacter.IsDead?` _ash2o_default_third_person_character))
    (bind _ash20_default_third_person_player_controller (cast `/Game/Blueprints/Gameplay/H20_DefaultThirdPersonPlayerController` _returnvalue_2))
    (if (`Controller.IsLocalController` _returnvalue_2)
      (bind _returnvalue_3 (`|CreateWidget` (`self.HitMarkerUI`) _ash20_default_third_person_player_controller))
      (`UserWidget.AddToPlayerScreen` _returnvalue_3 0)
      (if (not (`/Game/Blueprints/Scoring/H2O_PlayerState-CS.KillPlayer?` (cast `/Game/Blueprints/Scoring/H2O_PlayerState-CS` (`Pawn.PlayerState` _ash2o_default_third_person_character) :!pure true)))
        (`GameplayStatics.PlaySound2D` "/Game/Assets/Audio/SoundEffects/Hitmarker/H20_SFX_WaterGunShootHitGrass_10_v1_MSTD_AG.H20_SFX_WaterGunShootHitGrass_10_v1_MSTD_AG" 0.3 2.0 0.0 null _returnvalue)))))

(event `OnExplosion`
  ;[1 1 1] Explosion Effect
  (`GameplayStatics.SpawnEmitterAtLocation` (`self.ExplosionEffects`) (`self.K2_GetActorLocation`))
  (`self.SetActorEnableCollision` false)
  (`self.SetActorHiddenInGame` true))

(fn `ApplyWaterExplosionDamage`
  ;[1 1 1] Find all the players in the radius and does damage to them
  (bind _outactors (`KismetSystemLibrary.SphereOverlapActors` (`self.K2_GetActorLocation`) (`self.WaterExplosionRadius`) (`|MakeArray` "ObjectTypeQuery3" "ObjectTypeQuery6" :!type "EObjectTypeQuery Enum")))
  (for _array_element _outactors
    (`GameplayStatics.ApplyDamage` _array_element (`self.WaterExplosionDamage`) (`self.GetInstigatorController`) self)))

(fn `OnWaterBombLive`
  (bind _spherecollision (`self.SphereCollision`))
  ;[1 1 1] Server Handles Water Bomb Events
  (`/Engine/EditorBlueprintResources/ActorMacros.Switch Has Authority`
    (:`Authority`
      (`self.ApplyWaterExplosionDamage`)
      (`self.OnExplosion`)
      (`PrimitiveComponent.SetCollisionEnabled` _spherecollision "NoCollision")
      (`PrimitiveComponent.SetCollisionResponseToAllChannels` _spherecollision "ECR_Ignore")
      (`SceneComponent.SetHiddenInGame` (`self.WaterBombMesh`) false false)
      (`self.SetLifeSpan` 1.0))))

(fn `UserConstructionScript`)