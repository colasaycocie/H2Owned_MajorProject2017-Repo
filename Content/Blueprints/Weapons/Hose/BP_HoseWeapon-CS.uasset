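; BP_HoseWeapon is a possessable hose weapon that the player takes control of by walking into its sphere.
; On overlap, a third-person character with CanPossess set has its player controller possess the hose, and that character's movement is disabled.
; MoveForward and Turn share a yaw rotation, and LookUp drives pitch.
; Shoot and Reload only print debug text, and no release logic exists.
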(event `InputAxis|MoveForward`
  (params (AxisValue :type "Float (single-precision)"))
  (`self.K2_AddActorLocalRotation` (`KismetMathLibrary.MakeRotator` 0.0 0.0 AxisValue) :!label _label)
  (`KismetSystemLibrary.PrintString` (`KismetStringLibrary.Conv_DoubleToString` AxisValue)))

(event `InputAxis|Turn`
  (params (AxisValue :type "Float (single-precision)"))
  (goto _label))

(event `InputAction|Shoot`
  (params (Key :type "Key Structure"))
  (:`Pressed`
    (`KismetSystemLibrary.PrintString` "Hello")))

(event `InputAction|Reload`
  (params (Key :type "Key Structure"))
  (:`Pressed`
    (`KismetSystemLibrary.PrintString` "Hello")))

(event `InputAxis|LookUp`
  (params (AxisValue :type "Float (single-precision)"))
  (`self.K2_AddActorLocalRotation` (`KismetMathLibrary.MakeRotator` 0.0 AxisValue)))

(event `self.ReceiveTick`
  (params (DeltaSeconds :type "Float (single-precision)")))

(event `InputAction|InteractObjects`
  (params (Key :type "Key Structure")))

(event `self.Sphere.OnComponentBeginOverlap`
  (params (OverlappedComponent :type "PrimitiveComponent Object Reference") (OtherActor :type "Actor Object Reference") (OtherComp :type "PrimitiveComponent Object Reference") (OtherBodyIndex :type Integer) (bFromSweep :type Boolean) (SweepResult :type "HitResult Structure (by ref)"))
  (bind _ash2o_default_third_person_character (cast `/Game/Blueprints/Characters/H2O_Default_ThirdPersonCharacter` OtherActor))
  (if (`/Game/Blueprints/Characters/H2O_Default_ThirdPersonCharacter.CanPossess?` _ash2o_default_third_person_character)
    (bind _ash20_default_third_person_player_controller (cast `/Game/Blueprints/Gameplay/H20_DefaultThirdPersonPlayerController` (`self.GetController` _ash2o_default_third_person_character)))
    (`Controller.Possess` _ash20_default_third_person_player_controller self)
    (`Controller.Possess` (`self.GetController` _ash2o_default_third_person_character) self)
    (`CharacterMovementComponent.DisableMovement` (`Character.CharacterMovement` _ash2o_default_third_person_character))))

(event `self.Sphere.OnComponentEndOverlap`
  (params (OverlappedComponent :type "PrimitiveComponent Object Reference") (OtherActor :type "Actor Object Reference") (OtherComp :type "PrimitiveComponent Object Reference") (OtherBodyIndex :type Integer)))

(fn `UserConstructionScript`)