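; Base water gun weapon Blueprint that fires BP_WaterGunProjectile, still at a prototype stage.
; WeaponFire calls TestFire, which on authority spawns a projectile offset from player 0's capsule along third-person camera rotation.
; OnRep_isShooting duplicates that spawn, and both are marked for removal.
; Fire is empty, StopWeaponFire only prints, and the muzzle-socket spawn with explosion effect is disconnected.
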(event `Fire`)

(event `WeaponFire`
  (`KismetSystemLibrary.PrintString` "Firing")
  (`self.TestFire`))

(event `StopWeaponFire`
  (`KismetSystemLibrary.PrintString` "Not Fire"))

(fn `OnRep_isShooting`
  (bind _ash2o_default_third_person_character (cast `/Game/Blueprints/Characters/H2O_Default_ThirdPersonCharacter` (`GameplayStatics.GetPlayerCharacter` 0) :!pure true))
  (bind _returnvalue (`SceneComponent.K2_GetComponentRotation` (`/Game/Blueprints/Characters/H2O_Default_ThirdPersonCharacter.ThirdPersonCamera` _ash2o_default_third_person_character)))
  ;[1 1 1] This will be removed
  (`/Engine/EditorBlueprintResources/ActorMacros.Switch Has Authority`
    (:`Authority`
      (`|SpawnActorFromClass` "/Game/Blueprints/Weapons/BP_WaterGunProjectile.BP_WaterGunProjectile_C" (`KismetMathLibrary.MakeTransform` (+ (`SceneComponent.K2_GetComponentLocation` (`Character.CapsuleComponent` _ash2o_default_third_person_character)) (`KismetMathLibrary.GreaterGreater_VectorRotator` (100.0 0.0 50.0) _returnvalue)) _returnvalue) "Undefined" "OverrideRootScale" null null))))

(fn `TestFire`
  (bind _ash2o_default_third_person_character (cast `/Game/Blueprints/Characters/H2O_Default_ThirdPersonCharacter` (`GameplayStatics.GetPlayerCharacter` 0) :!pure true))
  (bind _returnvalue (`SceneComponent.K2_GetComponentRotation` (`/Game/Blueprints/Characters/H2O_Default_ThirdPersonCharacter.ThirdPersonCamera` _ash2o_default_third_person_character)))
  ;[1 1 1] This will be removed
  (`/Engine/EditorBlueprintResources/ActorMacros.Switch Has Authority`
    (:`Authority`
      (`|SpawnActorFromClass` "/Game/Blueprints/Weapons/BP_WaterGunProjectile.BP_WaterGunProjectile_C" (`KismetMathLibrary.MakeTransform` (+ (`SceneComponent.K2_GetComponentLocation` (`Character.CapsuleComponent` _ash2o_default_third_person_character)) (`KismetMathLibrary.GreaterGreater_VectorRotator` (100.0 0.0 50.0) _returnvalue)) _returnvalue) "Undefined" "OverrideRootScale" null null))))

(fn `UserConstructionScript`)