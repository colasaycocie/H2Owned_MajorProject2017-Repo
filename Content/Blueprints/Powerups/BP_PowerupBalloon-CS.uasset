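; Floating balloon pickup container that pops under damage and leaves a random power-up in its place.
; A timeline started on BeginPlay drifts the static mesh by adding its offsets to the world location each update.
; On authority, incoming damage accumulates in CurrentHealth until a threshold triggers the pop sound event, spawns a class from PowerUpArray and destroys the balloon.
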(event `self.ReceiveBeginPlay`
  (bind _staticmesh (`self.StaticMesh`))
  ;[1 1 1] Floating Animation
  (bind (_direction _movex _movez _movey) (`Timeline|Floating`)
    (:`Update`
      (`SceneComponent.K2_SetWorldLocation` _staticmesh (`KismetMathLibrary.MakeVector` (+ _movex (.x (`SceneComponent.K2_GetComponentLocation` _staticmesh))) (+ _movey (.y (`SceneComponent.K2_GetComponentLocation` _staticmesh))) (+ _movez (.z (`SceneComponent.K2_GetComponentLocation` _staticmesh)))) false false))))

(event `self.ReceiveAnyDamage`
  (params (Damage :type "Float (single-precision)") (DamageType :type "DamageType Object Reference") (InstigatedBy :type "Controller Object Reference") (DamageCauser :type "Actor Object Reference"))
  (bind _poweruparray (`self.PowerUpArray`))
  ;[1 1 1] Checks Balloon health, if it gets damaged more than 5, it will spawn a random power up
  (`/Engine/EditorBlueprintResources/ActorMacros.Switch Has Authority`
    (:`Authority`
      (bind _output_get (set `self.CurrentHealth` (+ (`self.CurrentHealth`) Damage)))
      (if (>= _output_get 5.0)
        ;[0.2518 1 0] Sound Effect
        (`self.ServerPlayBalloonPopSFX`)
        ;[1 1 1] Spawns random power up in the array
        (bind _returnvalue (`|SpawnActorFromClass` (`|GetArrayItem` _poweruparray (`KismetMathLibrary.RandomInteger` (`KismetArrayLibrary.Array_Length` _poweruparray))) (`KismetMathLibrary.Conv_VectorToTransform` (`self.K2_GetActorLocation`)) "Undefined" "OverrideRootScale" null null))
        (set `self.PowerupRef` _returnvalue)
        (`self.K2_DestroyActor`)))))

(event `ServerPlayBalloonPopSFX`
  ;[0.2518 1 0] Sound Effect
  (`GameplayStatics.PlaySoundAtLocation` "/Game/Assets/Audio/Powerups/PowerupBalloonPop/SFX_BalloonPop_Cue-CS.SFX_BalloonPop_Cue-CS" (`self.K2_GetActorLocation`)))

(fn `UserConstructionScript`)