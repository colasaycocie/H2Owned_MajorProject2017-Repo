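; BP_WaterGunProjectile is a water bomb projectile that explodes on its first bounce or expires after a fixed life span.
; On the server, the bounce calls OnWaterBombLive, which damages actors in a sphere overlap, triggers OnExplosion, and shortens the life span.
; OnExplosion spawns particles, disables collision and hides the actor.
; The hit handler is empty, and the fuse timer and explosion sound are unwired.
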(event `self.ReceiveBeginPlay`
  (`self.SetLifeSpan` 8.0) ; Life Span of the water bomb
)

(event `self.SphereCollision.OnComponentHit`
  (params (HitComponent :type "PrimitiveComponent Object Reference") (OtherActor :type "Actor Object Reference") (OtherComp :type "PrimitiveComponent Object Reference") (NormalImpulse :type "Vector Structure") (Hit :type "HitResult Structure (by ref)"))
  ;[0.8103 0.08215 0.0499] Hit Event / Need to figure out 90% chance of it exploding
)

(event `self.ProjectileMovement.OnProjectileBounce`
  (params (ImpactResult :type "HitResult Structure (by ref)") (ImpactVelocity :type "Vector Structure (by ref)"))
  ;[0.8103 0.08215 0.0499] Hit Event / Need to figure out 90% chance of it exploding
  (`/Engine/EditorBlueprintResources/ActorMacros.Switch Has Authority`
    (:`Authority`
      (`self.OnWaterBombLive`))))

(event `OnExplosion`
  ;[1 1 1] Explosion Effect
  (`GameplayStatics.SpawnEmitterAtLocation` (`self.ExplosionEffects`) (`self.K2_GetActorLocation`))
  (`self.SetActorEnableCollision` false)
  (`self.SetActorHiddenInGame` true))

(fn `ApplyWaterExplosionDamage`
  ;[1 1 1] Find all the players in the radius and does damage to them
  (bind _outactors (`KismetSystemLibrary.SphereOverlapActors` (`self.K2_GetActorLocation`) (`self.WaterExplosionRadius`) (`|MakeArray` "ObjectTypeQuery3" "ObjectTypeQuery1" :!type "EObjectTypeQuery Enum")))
  (for _array_element _outactors
    (`GameplayStatics.ApplyDamage` _array_element (`self.WaterExplosionDamage`) (`self.GetInstigatorController`) self)))

(fn `OnWaterBombLive`
  ;[1 1 1] Server Handles Water Bomb Events
  (`/Engine/EditorBlueprintResources/ActorMacros.Switch Has Authority`
    (:`Authority`
      (`self.ApplyWaterExplosionDamage`)
      (`self.OnExplosion`)
      (`self.SetLifeSpan` 1.0))))

(fn `UserConstructionScript`)